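; BP_EX03_2 is an exercise actor that moves continuously along the world X or Y axis according to a stored direction.
; MoveActor stores the incoming direction in CurrentDir and sets ChangeDir to false on both branches of its comparison.
; Tick switches on CurrentDir, offsetting location by MoveVal scaled by delta time: T/G for ±X, H/F for ±Y, while Space holds position.
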(event `self.ReceiveTick`
  (params (DeltaSeconds :type "Float (single-precision)"))
  (bind (_returnvalue_x _returnvalue_y) (`KismetMathLibrary.BreakVector` (`self.K2_GetActorLocation`)))
  (bind (_returnvalue_x_2 _returnvalue_y_2) (`KismetMathLibrary.BreakVector` (`self.K2_GetActorLocation`)))
  (bind (_returnvalue_x_3 _returnvalue_y_3) (`KismetMathLibrary.BreakVector` (`self.K2_GetActorLocation`)))
  (bind (_returnvalue_x_4 _returnvalue_y_4) (`KismetMathLibrary.BreakVector` (`self.K2_GetActorLocation`)))
  (set `self.Delta Seconds` DeltaSeconds)
  (switch `/Game/EX03/Direction` (`self.CurrentDir`)
    (:`NewEnumerator0`
      (`self.K2_SetActorLocation` (`KismetMathLibrary.MakeVector` (+ (* (`self.Delta Seconds`) (`self.MoveVal`)) _returnvalue_x_4) _returnvalue_y_4)))
    (:`NewEnumerator1`
      (`self.K2_SetActorLocation` (`KismetMathLibrary.MakeVector` (+ (* (* (`self.Delta Seconds`) (`self.MoveVal`)) -1.0) _returnvalue_x) _returnvalue_y)))
    (:`NewEnumerator2`
      (`self.K2_SetActorLocation` (`KismetMathLibrary.MakeVector` _returnvalue_x_2 (+ (* (* (`self.Delta Seconds`) (`self.MoveVal`)) -1.0) _returnvalue_y_2))))
    (:`NewEnumerator3`
      (`self.K2_SetActorLocation` (`KismetMathLibrary.MakeVector` _returnvalue_x_3 (+ (* (`self.Delta Seconds`) (`self.MoveVal`)) _returnvalue_y_3))))
    (:`NewEnumerator8`
      (`self.K2_SetActorLocation` (`self.K2_GetActorLocation`)))))

(fn `MoveActor`
  (params (InDir :type "/Game/EX03/Direction Enum" :default "NewEnumerator0"))
  (if (`|EnumInequality` InDir (`self.CurrentDir`))
    (set `self.ChangeDir` false)
    (else
      (set `self.ChangeDir` false)))
  (set `self.CurrentDir` (`local.InDir`)))

(fn `UserConstructionScript`)