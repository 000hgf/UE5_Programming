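; BP_Actor01 is a simple exercise actor that prints its own identity and transform on screen when play begins.
; BeginPlay prints the display name, then location, rotation and scale as separate strings, with location and rotation in distinct colors, all sharing a PrintDuration variable.
; The overlap and Tick events and the construction script are empty, and a few leftover nodes are unused.
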(event `self.ReceiveBeginPlay`
  (bind _printduration (`self.PrintDuration`))
  (bind (_returnvalue_location _returnvalue_rotation _returnvalue_scale) (`KismetMathLibrary.BreakTransform` (`self.GetTransform` self)))
  (`KismetSystemLibrary.PrintString` (`KismetSystemLibrary.GetDisplayName` self) true true (struct :`G` 0.66 :`B` 1.0 :`A` 1.0) _printduration)
  (`KismetSystemLibrary.PrintString` (`KismetStringLibrary.Conv_VectorToString` _returnvalue_location) true true (struct :`R` 1.0 :`G` 0.044178 :`A` 1.0) _printduration)
  (`KismetSystemLibrary.PrintString` (`KismetStringLibrary.Conv_RotatorToString` _returnvalue_rotation) true true (struct :`G` 1.0 :`B` 0.048798 :`A` 1.0) _printduration)
  (`KismetSystemLibrary.PrintString` (`KismetStringLibrary.Conv_VectorToString` _returnvalue_scale) true true (struct :`G` 0.66 :`B` 1.0 :`A` 1.0) _printduration))

(fn `UserConstructionScript`)