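; BP_MyGameState tracks the remaining coin count for the EX05 game and ends the round when it runs out.
; GetCoin exposes the count, and DecreaseCoinCount lowers it by one while it is above zero, then pushes it to the UMGCoinInfo widget.
; At zero it opens level L_EX05, a check that only runs when the widget reference is valid.
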(fn `DecreaseCoinCount`
  (bind _umgcoininfo (`self.UMGCoinInfo`))
  (if (> (`self.CoinCount`) 0)
    (set `self.CoinCount` (- (`self.CoinCount`) 1))
    (`/Engine/EditorBlueprintResources/StandardMacros.IsValid` _umgcoininfo
      (:`Is Valid`
        (`/Game/EX05/UMG/UI_Coininfo.SetRemainCoinCount` _umgcoininfo (`self.CoinCount`))
        (if (<= (`self.CoinCount`) 0)
          (`GameplayStatics.OpenLevelBySoftObjectPtr` "/Game/EX05/L_EX05.L_EX05"))))))

(fn `GetCoin`
  (returns (NewParam :type Integer))
  (return (`self.CoinCount`)))

(fn `UserConstructionScript`)