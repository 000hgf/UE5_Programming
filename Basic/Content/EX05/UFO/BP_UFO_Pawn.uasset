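; BP_UFO_Pawn is a player-controlled UFO pawn driven by Enhanced Input.
; On BeginPlay it adds the IMC_UFO mapping context to the local player's input subsystem.
; IA_MoveUFO adds movement input along the actor's forward vector when a controller is valid, and IA_LookUFO feeds yaw and pitch into controller rotation.
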(event `self.ReceiveBeginPlay`
  (bind `_as플레이어_컨트롤러` (cast `PlayerController` (`self.GetController`)))
  (`EnhancedInputSubsystemInterface.AddMappingContext` (pcsubsystem `EnhancedInputLocalPlayerSubsystem` `_as플레이어_컨트롤러`) "/Game/EX05/UFO/Input/IMC_UFO.IMC_UFO" 0 (struct)))

(event `EnhancedInput|/Game/EX05/UFO/Input/IA_MoveUFO`
  (params (ActionValue :type "Float (double-precision)") (ElapsedSeconds :type "Float (double-precision)") (TriggeredSeconds :type "Float (double-precision)") (InputAction :type "InputAction Object Reference" :default "/Game/EX05/UFO/Input/IA_MoveUFO.IA_MoveUFO"))
  (:`Triggered`
    (`/Engine/EditorBlueprintResources/StandardMacros.IsValid` (`self.GetController`)
      (:`Is Valid`
        (`self.AddMovementInput` (`self.GetActorForwardVector`) ActionValue)))))

(event `EnhancedInput|/Game/EX05/UFO/Input/IA_LookUFO`
  (params (ActionValue :type "Vector2D Structure") (ElapsedSeconds :type "Float (double-precision)") (TriggeredSeconds :type "Float (double-precision)") (InputAction :type "InputAction Object Reference" :default "/Game/EX05/UFO/Input/IA_LookUFO.IA_LookUFO"))
  (:`Triggered`
    (`self.AddControllerYawInput` ActionValue_X)
    (`self.AddControllerPitchInput` ActionValue_Y)))

(fn `UserConstructionScript`)