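; BP_Star is a star actor for the EX05 solar system that spins on its own axis.
; On BeginPlay it creates a dynamic material instance from SourceMaterial on the Star component's first material slot.
; Each Tick, while IsRotation is true, it adds relative yaw to Star at RotationSpeed scaled by delta time, keeping the spin frame-rate independent.
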(event `self.ReceiveBeginPlay`
  (`PrimitiveComponent.CreateDynamicMaterialInstance` (`self.Star`) 0 (`self.Source Material`) "None"))

(event `self.ReceiveTick`
  (params (DeltaSeconds :type "Float (single-precision)"))
  (if (`self.IsRotation`)
    ;[1 1 1] 자전
    (`SceneComponent.K2_AddRelativeRotation` (`self.Star`) (`KismetMathLibrary.MakeRotator` 0.0 0.0 (* DeltaSeconds (`self.RotationSpeed`))) false false)))

(fn `UserConstructionScript`)