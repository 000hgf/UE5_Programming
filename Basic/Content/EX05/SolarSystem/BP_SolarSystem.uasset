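; BP_SolarSystem is an actor that models a simple Sun, Earth and Moon system.
; The construction script sets the world scale of each body from its own scale variable.
; Tick yaws the Sun axis component at a constant, delta-time-scaled rate.
; A faster local rotation for the Earth axis is present but disconnected, so it never runs.
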(event `self.ReceiveTick`
  (params (DeltaSeconds :type "Float (single-precision)"))
  (`SceneComponent.K2_AddRelativeRotation` (`self.AxisSun`) (`KismetMathLibrary.MakeRotator` 0.0 0.0 (* DeltaSeconds 10.0)) false false))

(fn `UserConstructionScript`
  (`SceneComponent.SetWorldScale3D` (`self.Sun`) (`self.SunScale`))
  (`SceneComponent.SetWorldScale3D` (`self.Earth`) (`self.EarthScale`))
  (`SceneComponent.SetWorldScale3D` (`self.Moon`) (`self.MoonScale`)))