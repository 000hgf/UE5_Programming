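; UFO actor that spins continuously around one local axis, chosen by its Type setting.
; Tick stores the delta time and switches on Type to call one of six functions for positive or negative roll, pitch or yaw.
; Each function adds a local rotation scaled by Speed and delta time, so the spin is frame-rate independent.
; Disconnected SetActorRotation nodes in each function are unused alternatives that never run.
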(event `self.ReceiveTick`
  (params (DeltaSeconds :type "Float (single-precision)"))
  (set `self.ActorDeltaSecond` DeltaSeconds)
  (switch `/Game/EX04/E_Rotation` (`self.Type`)
    (:`NewEnumerator0`
      (`self.RollPlus`))
    (:`NewEnumerator1`
      (`self.RollMinus`))
    (:`NewEnumerator2`
      (`self.PitchPlus`))
    (:`NewEnumerator3`
      (`self.PitchMinus`))
    (:`NewEnumerator4`
      (`self.YawPlus`))
    (:`NewEnumerator5`
      (`self.YawMinus`))))

(fn `PitchMinus`
  (`self.K2_AddActorLocalRotation` (`KismetMathLibrary.MakeRotator` 0.0 (* (* (`self.ActorDeltaSecond`) (`self.Speed`)) -1.0))))

(fn `PitchPlus`
  (`self.K2_AddActorLocalRotation` (`KismetMathLibrary.MakeRotator` 0.0 (* (`self.ActorDeltaSecond`) (`self.Speed`)))))

(fn `RollMinus`
  (`self.K2_AddActorLocalRotation` (`KismetMathLibrary.MakeRotator` (* (* (`self.ActorDeltaSecond`) (`self.Speed`)) -1.0))))

(fn `RollPlus`
  (`self.K2_AddActorLocalRotation` (`KismetMathLibrary.MakeRotator` (* (`self.ActorDeltaSecond`) (`self.Speed`)))))

(fn `UserConstructionScript`)

(fn `YawMinus`
  (`self.K2_AddActorLocalRotation` (`KismetMathLibrary.MakeRotator` 0.0 0.0 (* (* (`self.ActorDeltaSecond`) (`self.Speed`)) -1.0))))

(fn `YawPlus`
  (`self.K2_AddActorLocalRotation` (`KismetMathLibrary.MakeRotator` 0.0 0.0 (* (`self.ActorDeltaSecond`) (`self.Speed`)))))